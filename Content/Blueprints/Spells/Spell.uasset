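; Base spell projectile actor that damages enemies it overlaps.
; On overlap it calls DealDamageAndDestroy, which ignores Player and Projectile tagged actors, applies its damage and type to Enemy tagged actors, and destroys itself on any other hit.
; The logic sits in its own function with an optional destroy flag and a success return, so child spells such as meteor can override it.
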(event EventActorBeginOverlap
  (params (OtherActor :type Actor%20Object%20Reference))
  ;[1 1 1] This is in its own function because sometimes other spells override it (e.g. meteor overrides to spawn ashes
  (CallFunction|DealDamageandDestroy OtherActor true))

(fn ConstructionScript)

(fn DealDamageandDestroy
  (params (Other%20Actor :type Actor%20Object%20Reference) (DestroyAtEnd :type Boolean))
  (if (Actor|ActorHasTag Other%20Actor "Player")
    (LocalVariables|SetSuccessful false :!label _label)
    (elif (Actor|ActorHasTag Other%20Actor "Projectile")
      (goto _label)
      (else
        (if (Actor|ActorHasTag Other%20Actor "Enemy")
          (Game|Damage|ApplyDamage Other%20Actor (Variables|Default|GetBaseDamage) 0 0 "/Script/Engine.DamageType"))
        (LocalVariables|SetSuccessful true)
        (if DestroyAtEnd
          (Actor|DestroyActor)))))
  (return (LocalVariables|GetSuccessful)))