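; Player character for a 2D side-scrolling spellcaster, with axis movement, jumping and flipbook animation chosen by a simple state function.
; Four attack inputs share one cast path that spawns a hardcoded spell class, deducts its mana and adds its experience to the matching elemental skill-tree bar.
; Damage and mana use update the HUD bars, while I and P toggle the skill-tree widget component and spellbook.
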(event Custom|UpdateAnimation
  ;[1 1 1] Animation(Idle,Running,Jumping)
  (Variables|Default|SetIsMoving (> (Math|Vector|VectorLength (Transformation|GetVelocity)) 0.0))
  (Variables|Default|SetIsFalling (AI|Components|NavMovement|IsFalling (Variables|Character|GetCharacterMovement)))
  (bind _outputflipbook (CallFunction|AnimationStateMachine (Variables|Default|GetIsFalling) (Variables|Default|GetIsMoving)))
  (Sprite|SetFlipbook (Variables|Default|GetSprite) _outputflipbook))

(event EventAnyDamage
  (params (Damage :type Float%20%28single-precision%29) (DamageType :type Damage%20Type%20Object%20Reference) (InstigatedBy :type Controller%20Object%20Reference) (DamageCauser :type Actor%20Object%20Reference))
  ;[1 1 1] Player took damage, calculate new health
  (Variables|Default|SetPlayerHealth (- (Variables|Default|GetPlayerHealth) Damage))
  (Development|PrintString "I have been damaged")
  (bind _asui (Utilities|Casting|CastToUI (Variables|Default|GetUI)))
  (Progress|SetPercent (Variables|/Game/UI/HUD/UI.UI_C|GetMHealthBar _asui) (/ (Variables|Default|GetPlayerHealth) 2e+02)))

(event EventBeginPlay
  ;[1 1 1] BEGIN PLAY
  (Rendering|ToggleVisibility false)
  (Transformation|AddWorldOffset "500.000000, 0, 0" false)
  ;[1 1 1] Show Mouse cursor
  (Variables|/Script/Engine.PlayerController|SetbShowMouseCursor (Game|GetPlayerController 0) true)
  ;[1 1 1] Set up spell classes assigned to abilities 1, 2, 3 ,4. Hardcoded for now, but these classes will change as player changes spells
  (Variables|Default|SetSpell1Class "/Game/Blueprints/Spells/FireBall.Fireball_C")
  (Variables|Default|SetSpell2Class "/Game/Blueprints/Spells/WaterBolt.Waterbolt_C")
  (Variables|Default|SetSpell3Class "/Game/Blueprints/Spells/Leafstrike.Leafstrike_C")
  (Variables|Default|SetSpell4Class "/Game/Blueprints/Spells/Airblast.Airblast_C")
  ;[1 1 1] Spawn the UI
  (bind _returnvalue (UserInterface|CreateWidget "/Game/UI/HUD/UI.UI_C"))
  (bind _output_get (Variables|Default|SetUI _returnvalue))
  (UserInterface|Viewport|AddtoViewport _output_get 0))

(event Input|ActionEvents|InputActionJump
  ;[1 1 1] Jumping
  (:Pressed
    (Character|Jump)))

(event Input|ActionEvents|InputActionBasicAttack
  ;[1 1 1] Spell Attacks
  (:Pressed
    (Variables|Default|SetCurrentSpellClass (Variables|Default|GetSpell1Class))
    (bind (_manaused _outputspelltype _outputexp) (CallFunction|SpellCast (Variables|Default|GetCurrentSpellClass)))
    (Variables|Default|Setcurrentspelltype _outputspelltype)
    (Variables|Default|Setoutputexp _outputexp)
    ;[1 1 1] Mana Usage
    (Variables|Default|SetPlayerMana (- (Variables|Default|GetPlayerMana) _manaused))
    (bind _asui (Utilities|Casting|CastToUI (Variables|Default|GetUI)))
    (Progress|SetPercent (Variables|/Game/UI/HUD/UI.UI_C|GetMManaBar _asui) (/ (Variables|Default|GetPlayerMana) 1e+02))
    ;[1 1 1] Skill Tree Expereince
    (switch Utilities|FlowControl|Switch|SwitchonSpellTypes (Variables|Default|Getcurrentspelltype)
      (:NewEnumerator0
        ;;[1 1 1] Attack Layer
        (|SetPercentUI_FireA))
      (:NewEnumerator3
        (|SetPercentUI_EarthA))
      (:NewEnumerator6
        (|SetPercentUI_WaterA))
      (:NewEnumerator9
        (|SetPercentUI_AirA)))))

(event Input|ActionEvents|InputActionBasicAttack2
  ;[1 1 1] Spell Attacks
  (:Pressed
    (Variables|Default|SetCurrentSpellClass (Variables|Default|GetSpell2Class))
    (bind (_manaused _outputspelltype _outputexp) (CallFunction|SpellCast (Variables|Default|GetCurrentSpellClass)))
    (Variables|Default|Setcurrentspelltype _outputspelltype)
    (Variables|Default|Setoutputexp _outputexp)
    ;[1 1 1] Mana Usage
    (Variables|Default|SetPlayerMana (- (Variables|Default|GetPlayerMana) _manaused))
    (bind _asui (Utilities|Casting|CastToUI (Variables|Default|GetUI)))
    (Progress|SetPercent (Variables|/Game/UI/HUD/UI.UI_C|GetMManaBar _asui) (/ (Variables|Default|GetPlayerMana) 1e+02))
    ;[1 1 1] Skill Tree Expereince
    (switch Utilities|FlowControl|Switch|SwitchonSpellTypes (Variables|Default|Getcurrentspelltype)
      (:NewEnumerator0
        ;;[1 1 1] Attack Layer
        (|SetPercentUI_FireA))
      (:NewEnumerator3
        (|SetPercentUI_EarthA))
      (:NewEnumerator6
        (|SetPercentUI_WaterA))
      (:NewEnumerator9
        (|SetPercentUI_AirA)))))

(event Input|ActionEvents|InputActionBasicAttack3
  ;[1 1 1] Spell Attacks
  (:Pressed
    (Variables|Default|SetCurrentSpellClass (Variables|Default|GetSpell3Class))
    (bind (_manaused _outputspelltype _outputexp) (CallFunction|SpellCast (Variables|Default|GetCurrentSpellClass)))
    (Variables|Default|Setcurrentspelltype _outputspelltype)
    (Variables|Default|Setoutputexp _outputexp)
    ;[1 1 1] Mana Usage
    (Variables|Default|SetPlayerMana (- (Variables|Default|GetPlayerMana) _manaused))
    (bind _asui (Utilities|Casting|CastToUI (Variables|Default|GetUI)))
    (Progress|SetPercent (Variables|/Game/UI/HUD/UI.UI_C|GetMManaBar _asui) (/ (Variables|Default|GetPlayerMana) 1e+02))
    ;[1 1 1] Skill Tree Expereince
    (switch Utilities|FlowControl|Switch|SwitchonSpellTypes (Variables|Default|Getcurrentspelltype)
      (:NewEnumerator0
        ;;[1 1 1] Attack Layer
        (|SetPercentUI_FireA))
      (:NewEnumerator3
        (|SetPercentUI_EarthA))
      (:NewEnumerator6
        (|SetPercentUI_WaterA))
      (:NewEnumerator9
        (|SetPercentUI_AirA)))))

(event Input|ActionEvents|InputActionBasicAttack4
  ;[1 1 1] Spell Attacks
  (:Pressed
    (Variables|Default|SetCurrentSpellClass (Variables|Default|GetSpell4Class))
    (bind (_manaused _outputspelltype _outputexp) (CallFunction|SpellCast (Variables|Default|GetCurrentSpellClass)))
    (Variables|Default|Setcurrentspelltype _outputspelltype)
    (Variables|Default|Setoutputexp _outputexp)
    ;[1 1 1] Mana Usage
    (Variables|Default|SetPlayerMana (- (Variables|Default|GetPlayerMana) _manaused))
    (bind _asui (Utilities|Casting|CastToUI (Variables|Default|GetUI)))
    (Progress|SetPercent (Variables|/Game/UI/HUD/UI.UI_C|GetMManaBar _asui) (/ (Variables|Default|GetPlayerMana) 1e+02))
    ;[1 1 1] Skill Tree Expereince
    (switch Utilities|FlowControl|Switch|SwitchonSpellTypes (Variables|Default|Getcurrentspelltype)
      (:NewEnumerator0
        ;;[1 1 1] Attack Layer
        (|SetPercentUI_FireA))
      (:NewEnumerator3
        (|SetPercentUI_EarthA))
      (:NewEnumerator6
        (|SetPercentUI_WaterA))
      (:NewEnumerator9
        (|SetPercentUI_AirA)))))

(event Input|AxisEvents|InputAxisMoveRight
  (params (AxisValue :type Float%20%28single-precision%29))
  ;[1 1 1] Movement
  (Pawn|Input|AddMovementInput "1.000000, 0, 0" AxisValue false)
  (CallFunction|UpdateAnimation)
  (Math|Float|CompareFloat AxisValue 0.0
    (:>
      (Pawn|SetControlRotation (Pawn|GetController) (Class|KismetMathLibrary|MakeRot 0.0 0.0 0.0)))
    (:<
      (Pawn|SetControlRotation (Pawn|GetController) (Class|KismetMathLibrary|MakeRot 0.0 1.8e+02 0.0)))))

(event Input|KeyboardEvents|I
  ;[1 1 1] Open SkillTree menu
  (:Pressed
    (Utilities|FlowControl|FlipFlop
      (:A
        (Variables|Default|SetSkillsOpen true)
        (Transformation|AddWorldOffset "-500.000000, 0, 0" false))
      (:B
        (Variables|Default|SetSkillsOpen false)
        (Transformation|AddWorldOffset "500.000000, 0, 0" false)))
    (Rendering|ToggleVisibility (Variables|Default|GetWidget1) false)
    (Input|SetInputModeGameandUI (Game|GetPlayerController 0) 0 false false)))

(event Input|KeyboardEvents|P
  ;[1 1 1] Open SpellBook
  (:Pressed
    (Utilities|FlowControl|FlipFlop
      (:A
        (bind _returnvalue (UserInterface|CreateWidget "/Game/UI/SkillSystem/SpellBook.SpellBook_C"))
        (Widget|Transform|SetRenderScale _returnvalue "(X=0.400000,Y=0.400000)")
        (Class|Widget|SetRenderTranslation _returnvalue "(X=450.000000,Y=-300.000000)")
        (UserInterface|Viewport|AddtoViewport _returnvalue 0))
      (:B
        (Widget|RemovefromParent _returnvalue)))))

(fn ConstructionScript)

(fn AnimationStateMachine
  (params (IsFalling :type Boolean) (IsMoving :type Boolean))
  (LocalVariables|SetIsFallingLocal IsFalling)
  (LocalVariables|SetIsMovingLocal IsMoving)
  (if (LocalVariables|GetIsFallingLocal)
    (LocalVariables|SetAnimationState "NewEnumerator2")
    (elif (LocalVariables|GetIsMovingLocal)
      (LocalVariables|SetAnimationState "NewEnumerator1")
      (else
        (LocalVariables|SetAnimationState "NewEnumerator0"))))
  (return (Utilities|Select :Index (LocalVariables|GetAnimationState) :NewEnumerator0 "/Game/Flipbook/MainCharacter/MC_Idle.MC_Idle" :NewEnumerator1 "/Game/Flipbook/MainCharacter/MC_Running.MC_Running" :NewEnumerator2 "/Game/Flipbook/MainCharacter/MC_Idle.MC_Idle")))

(fn SpellCast
  (params (SpellClass :type Object%20Class%20Reference))
  (bind _asactor (Utilities|Casting|CastToActorClass SpellClass))
  (bind _returnvalue (Game|SpawnActorfromClass _asactor (|2DSpellTransform) false 0))
  (bind _asspell (Utilities|Casting|CastToSpell _returnvalue))
  (return (Variables|/Game/Blueprints/Spells/Spell.Spell_C|GetManaCost _asspell) (Variables|/Game/Blueprints/Spells/Spell.Spell_C|GetType _asspell) (Variables|/Game/Blueprints/Spells/Spell.Spell_C|GetExp _asspell)))